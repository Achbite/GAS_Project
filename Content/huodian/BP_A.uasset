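; Interactive prop that animates six pillars, six stones and a point light when the player presses the fakl input.
; A box overlap enables input and, for the third-person character, shows a widget; the end-overlap cleanup is unwired.
; A FlipFlop plays or reverses two timelines mapped to positions and light intensity.
; Opening also triggers a one-time level sequence via the character and, after a delay, UI-only widgets, which closing undoes.
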(event `self.Box.OnComponentBeginOverlap`
  (params (OverlappedComponent :type "PrimitiveComponent Object Reference") (OtherActor :type "Actor Object Reference") (OtherComp :type "PrimitiveComponent Object Reference") (OtherBodyIndex :type Integer) (bFromSweep :type Boolean) (SweepResult :type "HitResult Structure (by ref)"))
  (`self.EnableInput` (`GameplayStatics.GetPlayerController` 0))
  (cast `/Game/ThirdPerson/Blueprints/Character/BP_ThirdPersonCharacter` OtherActor)
  (bind _returnvalue (`|CreateWidget` null))
  (`UserWidget.AddToViewport` _returnvalue 0))

(event `self.ReceiveBeginPlay`
  (bind _asbp_third_person_character (cast `/Game/ThirdPerson/Blueprints/Character/BP_ThirdPersonCharacter` (`GameplayStatics.GetPlayerCharacter` 0)))
  (set `self.As BP Third Person Character` _asbp_third_person_character))

(event `playvideo`
  (bind _returnvalue (`GameplayStatics.GetPlayerController` 0))
  (bind _returnvalue_2 (`GameplayStatics.GetPlayerController` 0))
  (`/Engine/EditorBlueprintResources/StandardMacros.FlipFlop`
    (:`A`
      (`|ExecutionSequence`
        (:`then_0`
          (bind (_direction `_新建轨道_1`) (`Timeline|柱一` :!label _label)
            (:`Update`
              (`SceneComponent.K2_SetRelativeLocation` (`self.柱1`) (`KismetMathLibrary.MakeVector` (`KismetMathLibrary.MapRangeUnclamped` `_新建轨道_1` 0.0 1.0 -190.0 -210.0) 0.0 (`KismetMathLibrary.MapRangeUnclamped` `_新建轨道_1` 0.0 1.0 20.0 185.0)) false false)
              (`SceneComponent.K2_SetRelativeLocationAndRotation` :`self` (`self.柱2`) :`NewLocation` (`KismetMathLibrary.MakeVector` (`KismetMathLibrary.MapRangeUnclamped` `_新建轨道_1` 0.0 1.0 -105.0 -115.0) (`KismetMathLibrary.MapRangeUnclamped` `_新建轨道_1` 0.0 1.0 160.0 180.0) (`KismetMathLibrary.MapRangeUnclamped` `_新建轨道_1` 0.0 1.0 20.0 185.0)))
              (`SceneComponent.K2_SetRelativeLocationAndRotation` :`self` (`self.柱3`) :`NewLocation` (`KismetMathLibrary.MakeVector` (`KismetMathLibrary.MapRangeUnclamped` `_新建轨道_1` 0.0 1.0 105.0 115.0) (`KismetMathLibrary.MapRangeUnclamped` `_新建轨道_1` 0.0 1.0 160.0 180.0) (`KismetMathLibrary.MapRangeUnclamped` `_新建轨道_1` 0.0 1.0 20.0 185.0)))
              (`SceneComponent.K2_SetRelativeLocationAndRotation` :`self` (`self.柱4`) :`NewLocation` (`KismetMathLibrary.MakeVector` (`KismetMathLibrary.MapRangeUnclamped` `_新建轨道_1` 0.0 1.0 190.0 210.0) 0.0 (`KismetMathLibrary.MapRangeUnclamped` `_新建轨道_1` 0.0 1.0 20.0 185.0)))
              (`SceneComponent.K2_SetRelativeLocationAndRotation` :`self` (`self.柱5`) :`NewLocation` (`KismetMathLibrary.MakeVector` (`KismetMathLibrary.MapRangeUnclamped` `_新建轨道_1` 0.0 1.0 105.0 115.0) (`KismetMathLibrary.MapRangeUnclamped` `_新建轨道_1` 0.0 1.0 -160.0 -180.0) (`KismetMathLibrary.MapRangeUnclamped` `_新建轨道_1` 0.0 1.0 20.0 185.0)))
              (`SceneComponent.K2_SetRelativeLocationAndRotation` :`self` (`self.柱6`) :`NewLocation` (`KismetMathLibrary.MakeVector` (`KismetMathLibrary.MapRangeUnclamped` `_新建轨道_1` 0.0 1.0 -105.0 -115.0) (`KismetMathLibrary.MapRangeUnclamped` `_新建轨道_1` 0.0 1.0 -160.0 -180.0) (`KismetMathLibrary.MapRangeUnclamped` `_新建轨道_1` 0.0 1.0 20.0 185.0)))
              (`LightComponent.SetIntensity` (`self.PointLight`) (`KismetMathLibrary.MapRangeUnclamped` `_新建轨道_1` 0.0 1.0 0.0 5000.0)))))
        (:`then_1`
          (bind (_direction_2 `_新建轨道_1_2`) (`Timeline|时间轴_0` :!label _label_2)
            (:`Update`
              (`SceneComponent.K2_SetRelativeLocation` (`self.石1`) (`KismetMathLibrary.MakeVector` (`KismetMathLibrary.MapRangeUnclamped` `_新建轨道_1_2` 0.0 1.0 -190.0) (`KismetMathLibrary.MapRangeUnclamped` `_新建轨道_1_2` 0.0 1.0) (`KismetMathLibrary.MapRangeUnclamped` `_新建轨道_1_2` 0.0 1.0 90.0 70.0)) false false)
              (`SceneComponent.K2_SetRelativeLocationAndRotation` :`self` (`self.石2`) :`NewLocation` (`KismetMathLibrary.MakeVector` (`KismetMathLibrary.MapRangeUnclamped` `_新建轨道_1_2` 0.0 1.0 -105.0) (`KismetMathLibrary.MapRangeUnclamped` `_新建轨道_1_2` 0.0 1.0 160.0 100.0) (`KismetMathLibrary.MapRangeUnclamped` `_新建轨道_1_2` 0.0 1.0 90.0 95.0)))
              (`SceneComponent.K2_SetRelativeLocationAndRotation` :`self` (`self.石3`) :`NewLocation` (`KismetMathLibrary.MakeVector` (`KismetMathLibrary.MapRangeUnclamped` `_新建轨道_1_2` 0.0 1.0 105.0) (`KismetMathLibrary.MapRangeUnclamped` `_新建轨道_1_2` 0.0 1.0 160.0 100.0) (`KismetMathLibrary.MapRangeUnclamped` `_新建轨道_1_2` 0.0 1.0 90.0 150.0)))
              (`SceneComponent.K2_SetRelativeLocation` (`self.石4`) (`KismetMathLibrary.MakeVector` (`KismetMathLibrary.MapRangeUnclamped` `_新建轨道_1_2` 0.0 1.0 190.0) (`KismetMathLibrary.MapRangeUnclamped` `_新建轨道_1_2` 0.0 1.0) (`KismetMathLibrary.MapRangeUnclamped` `_新建轨道_1_2` 0.0 1.0 90.0 175.0)) false false)
              (`SceneComponent.K2_SetRelativeLocationAndRotation` :`self` (`self.石5`) :`NewLocation` (`KismetMathLibrary.MakeVector` (`KismetMathLibrary.MapRangeUnclamped` `_新建轨道_1_2` 0.0 1.0 105.0) (`KismetMathLibrary.MapRangeUnclamped` `_新建轨道_1_2` 0.0 1.0 -160.0 -100.0) (`KismetMathLibrary.MapRangeUnclamped` `_新建轨道_1_2` 0.0 1.0 90.0 150.0)))
              (`SceneComponent.K2_SetRelativeLocationAndRotation` :`self` (`self.石6`) :`NewLocation` (`KismetMathLibrary.MakeVector` (`KismetMathLibrary.MapRangeUnclamped` `_新建轨道_1_2` 0.0 1.0 -105.0) (`KismetMathLibrary.MapRangeUnclamped` `_新建轨道_1_2` 0.0 1.0 -160.0 -100.0) (`KismetMathLibrary.MapRangeUnclamped` `_新建轨道_1_2` 0.0 1.0 90.0 95.0))))))
        (:`then_2`
          (`/Engine/EditorBlueprintResources/StandardMacros.DoOnce` false
            (:`Completed`
              (`/Game/ThirdPerson/Blueprints/Character/BP_ThirdPersonCharacter.PlayLevelSequence` (`self.As BP Third Person Character`) null "None"))))
        (:`then_3`
          (`KismetSystemLibrary.Delay` 2.0)
          (`SceneComponent.SetVisibility` (`self.Widget`) true false)
          (bind _returnvalue_3 (`|CreateWidget` null))
          (`UserWidget.AddToViewport` _returnvalue_3 0)
          (set `PlayerController.bShowMouseCursor` true _returnvalue_2)
          (`WidgetBlueprintLibrary.SetInputMode_UIOnlyEx` _returnvalue_2 null))))
    (:`B`
      (`|ExecutionSequence`
        (:`then_0`
          (goto _label :!via `Reverse`))
        (:`then_1`
          (goto _label_2 :!via `Reverse`))
        (:`then_2`
          (`SceneComponent.SetVisibility` (`self.Widget`) false false)
          (`Widget.RemoveFromParent` _returnvalue_3)
          (set `PlayerController.bShowMouseCursor` false _returnvalue)
          (`WidgetBlueprintLibrary.SetInputMode_GameOnly` _returnvalue))))))

(event `InputAction|fakl`
  (params (Key :type "Key Structure"))
  (:`Pressed`
    (`self.playvideo`)))

(event `self.Box.OnComponentEndOverlap`
  (params (OverlappedComponent :type "PrimitiveComponent Object Reference") (OtherActor :type "Actor Object Reference") (OtherComp :type "PrimitiveComponent Object Reference") (OtherBodyIndex :type Integer)))

(fn `UserConstructionScript`)