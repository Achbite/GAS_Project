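; Dialogue component (对话组件) that opens and closes the on-screen dialogue UI from stored dialogue data.
; 开始对话 creates and displays a 对话界面 widget, hides the mouse cursor, copies the name, text and image from its dialogue struct into the widget, then calls its 对话 function.
; 结束对话 removes that widget, then also removes all top-level widgets of the same class from the screen.
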(event `开始对话`
  (bind `_对话ui` (`self.对话UI`))
  (bind (`_名字` `_对话内容` _img) (break `/Game/AllThing/BluePrints/对话系统/对话结构体` (`self.对话结构体变量`)))
  (bind _returnvalue (`|CreateWidget` "/Game/AllThing/BluePrints/对话系统/对话界面.对话界面_C"))
  (bind _output_get (set `self.对话UI` _returnvalue))
  (`UserWidget.AddToViewport` _output_get 0)
  (set `PlayerController.bShowMouseCursor` false (`GameplayStatics.GetPlayerController` 0))
  (set `/Game/AllThing/BluePrints/对话系统/对话界面.内容` (make `/Game/AllThing/BluePrints/对话系统/对话结构体` `_名字` `_对话内容` _img) `_对话ui`)
  (`/Game/AllThing/BluePrints/对话系统/对话界面.对话` `_对话ui`))

(event `结束对话`
  (`Widget.RemoveFromParent` (`self.对话UI`))
  (bind _foundwidgets (`WidgetBlueprintLibrary.GetAllWidgetsOfClass` "/Game/AllThing/BluePrints/对话系统/对话界面.对话界面_C"))
  (`Widget.RemoveFromParent` _foundwidgets))