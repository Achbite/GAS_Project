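; Health potion treasure chest that the third-person character opens by pressing F nearby, spawning potion pickups.
; One overlap sphere enables input and opens the gate; another toggles a prompt widget that turns toward the camera each tick.
; Opening plays a sound and a timeline rotating the lid, while a DoOnce hides the widget, spawns randomly yawed potions and destroys the chest after a short delay.
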(event `Key|F`
  (params (Key :type "Key Structure"))
  (:`Pressed`
    (`/Engine/EditorBlueprintResources/StandardMacros.Gate` true :!label _label
      (:`Exit`
        (`/Engine/EditorBlueprintResources/StandardMacros.DoOnce` false
          (:`Completed`
            (`GameplayStatics.PlaySound2D` "/Game/AllThing/Audio/开箱子声.开箱子声" 1.0 1.0 0.0 null null)
            (bind (_direction `_新建轨道_0`) (`Timeline|时间轴_0`)
              (:`Update`
                (`SceneComponent.K2_SetRelativeRotation` (`self.箱盖`) (`KismetMathLibrary.MakeRotator` 0.0 (`KismetMathLibrary.MapRangeUnclamped` `_新建轨道_0` 0.0 1.0 0.0 120.0)) false false)
                (`/Engine/EditorBlueprintResources/StandardMacros.DoOnce` false
                  (:`Completed`
                    (`SceneComponent.SetVisibility` (`self.Widget`) false false)
                    (set `self.组件已销毁` true)
                    (for _ (range 3)
                      (`|SpawnActorFromClass` "/Game/BackPack/Items/Items_hppotion.Items_hppotion_C" (`KismetMathLibrary.MakeTransform` (`self.K2_GetActorLocation` self) (`KismetMathLibrary.MakeRotator` 0.0 0.0 (`KismetMathLibrary.RandomFloatInRange` 0.0 180.0))) "AlwaysSpawn" "OverrideRootScale" null null)
                      (`KismetSystemLibrary.Delay` 1.5)
                      (`self.K2_DestroyActor` self))))))))))))

(event `self.Sphere.OnComponentBeginOverlap`
  (params (OverlappedComponent :type "PrimitiveComponent Object Reference") (OtherActor :type "Actor Object Reference") (OtherComp :type "PrimitiveComponent Object Reference") (OtherBodyIndex :type Integer) (bFromSweep :type Boolean) (SweepResult :type "HitResult Structure (by ref)"))
  (cast `/Game/ThirdPerson/Blueprints/Character/BP_ThirdPersonCharacter` OtherActor)
  (`self.EnableInput` (`GameplayStatics.GetPlayerController` 0))
  (goto _label :!via `Open`))

(event `self.Sphere.OnComponentEndOverlap`
  (params (OverlappedComponent :type "PrimitiveComponent Object Reference") (OtherActor :type "Actor Object Reference") (OtherComp :type "PrimitiveComponent Object Reference") (OtherBodyIndex :type Integer))
  (cast `/Game/ThirdPerson/Blueprints/Character/BP_ThirdPersonCharacter` OtherActor)
  (`self.DisableInput` (`GameplayStatics.GetPlayerController` 0)))

(event `self.Sphere1.OnComponentBeginOverlap`
  (params (OverlappedComponent :type "PrimitiveComponent Object Reference") (OtherActor :type "Actor Object Reference") (OtherComp :type "PrimitiveComponent Object Reference") (OtherBodyIndex :type Integer) (bFromSweep :type Boolean) (SweepResult :type "HitResult Structure (by ref)"))
  (cast `/Game/ThirdPerson/Blueprints/Character/BP_ThirdPersonCharacter` OtherActor)
  (if (not (`self.组件已销毁`))
    (`SceneComponent.SetVisibility` (`self.Widget`) true false)))

(event `self.Sphere1.OnComponentEndOverlap`
  (params (OverlappedComponent :type "PrimitiveComponent Object Reference") (OtherActor :type "Actor Object Reference") (OtherComp :type "PrimitiveComponent Object Reference") (OtherBodyIndex :type Integer))
  (cast `/Game/ThirdPerson/Blueprints/Character/BP_ThirdPersonCharacter` OtherActor)
  (if (not (`self.组件已销毁`))
    (`SceneComponent.SetVisibility` (`self.Widget`) false false)))

(event `self.ReceiveTick`
  (params (DeltaSeconds :type "Float (single-precision)"))
  (if (not (`self.组件已销毁`))
    (`SceneComponent.K2_SetWorldRotation` (`self.Widget`) (`KismetMathLibrary.FindLookAtRotation` (`SceneComponent.K2_GetComponentLocation` (`self.Widget`)) (`PlayerCameraManager.GetCameraLocation` (`GameplayStatics.GetPlayerCameraManager` 0))) false false)))

(fn `UserConstructionScript`)